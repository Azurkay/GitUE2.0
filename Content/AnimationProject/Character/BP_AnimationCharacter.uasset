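; BP_AnimationCharacter is a player character with Enhanced Input movement, look, jump, sprint and a pause menu toggle.
; Walk and Run set a target speed, which Tick eases MaxWalkSpeed toward with a fixed-alpha Lerp.
; Normalized stamina drains while sprint is held in motion and recovers on Tick otherwise, but never limits sprinting here.
; TogglePause lazily creates WBP_PauseMenu, then switches pause state, cursor and input mode.
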(event Custom|TogglePause
  (bind _returnvalue (Game|GetPlayerController 0))
  (bind _returnvalue_2 (Game|GetPlayerController 0))
  (if (Utilities|IsValid (Variables|UI|GetPauseUI))
    _
    (else
      ;[0 0 0] 1. Creation
      (bind _returnvalue_3 (UserInterface|CreateWidget "/Game/AnimationProject/UI/WBP_PauseMenu.WBP_PauseMenu_C"))
      (Variables|UI|SetPauseUI _returnvalue_3)))
  (if (UserInterface|Viewport|IsinViewport (Variables|UI|GetPauseUI))
    (Widget|RemovefromParent (Variables|UI|GetPauseUI))
    (Game|SetGamePaused false)
    (Variables|/Script/Engine.PlayerController|SetbShowMouseCursor _returnvalue_2 false)
    (Input|SetInputModeGameOnly _returnvalue false)
    (else
      (UserInterface|Viewport|AddtoViewport (Variables|UI|GetPauseUI) 0)
      (Game|SetGamePaused true)
      (Variables|/Script/Engine.PlayerController|SetbShowMouseCursor _returnvalue_2 true)
      (Input|SetInputModeGameandUI _returnvalue (Variables|UI|GetPauseUI) "DoNotLock" true false))))

(event Input|EnhancedActionEvents|EnhancedInputActionIA_Move
  (params (ActionValue :type Vector%202D%20Structure) (ElapsedSeconds :type Float%20%28double-precision%29) (TriggeredSeconds :type Float%20%28double-precision%29) (InputAction :type Input%20Action%20Object%20Reference :default "/Game/AnimationProject/Input/Action/IA_Move.IA_Move"))
  (bind _returnvalue (Pawn|GetControlRotation :!class /Script/Engine.Pawn))
  (Pawn|Input|AddMovementInput (Math|Vector|GetRightVector (Math|Rotator|MakeRotator 0.0 0.0 (.yaw _returnvalue))) (.x ActionValue) false)
  (Pawn|Input|AddMovementInput (Math|Vector|GetForwardVector (Math|Rotator|MakeRotator 0.0 0.0 (.yaw _returnvalue))) (.y ActionValue) false))

(event Input|EnhancedActionEvents|EnhancedInputActionIA_Look
  (params (ActionValue :type Vector%202D%20Structure) (ElapsedSeconds :type Float%20%28double-precision%29) (TriggeredSeconds :type Float%20%28double-precision%29) (InputAction :type Input%20Action%20Object%20Reference :default "/Game/AnimationProject/Input/Action/IA_Look.IA_Look"))
  (Pawn|Input|AddControllerYawInput (.x ActionValue))
  (Pawn|Input|AddControllerPitchInput (.y ActionValue)))

(event Input|EnhancedActionEvents|EnhancedInputActionIA_Jump
  (params (ActionValue :type Boolean) (ElapsedSeconds :type Float%20%28double-precision%29) (TriggeredSeconds :type Float%20%28double-precision%29) (InputAction :type Input%20Action%20Object%20Reference :default "/Game/AnimationProject/Input/Action/IA_Jump.IA_Jump"))
  (:Started
    (Character|Jump))
  (:Canceled
    (Character|StopJumping :!label _label))
  (:Completed
    (goto _label)))

(event Input|EnhancedActionEvents|EnhancedInputActionIA_Sprint
  (params (ActionValue :type Boolean) (ElapsedSeconds :type Float%20%28double-precision%29) (TriggeredSeconds :type Float%20%28double-precision%29) (InputAction :type Input%20Action%20Object%20Reference :default "/Game/AnimationProject/Input/Action/IA_Sprint.IA_Sprint"))
  (:Triggered
    ;[1 0 0] On perd de la stamina
    (Lose|LoseStaminaLogic))
  (:Started
    (Speed|Run))
  (:Canceled
    (Speed|Walk :!label _label))
  (:Completed
    (goto _label)))

(event Input|EnhancedActionEvents|EnhancedInputActionIA_Pause
  (params (ActionValue :type Boolean) (ElapsedSeconds :type Float%20%28double-precision%29) (TriggeredSeconds :type Float%20%28double-precision%29) (InputAction :type Input%20Action%20Object%20Reference :default "/Game/AnimationProject/Input/Action/IA_Pause.IA_Pause"))
  (:Started
    (CallFunction|TogglePause)))

(event EventTick
  (params (DeltaSeconds :type Float%20%28single-precision%29))
  ;[0 0.3854 0.01913] On récupère de la stamina
  (Recover|RecoverStaminaLogic)
  (Speed|SmoothChangeMaxWalkSpeed))

(event EventBeginPlay
  (Speed|Walk))

(fn ConstructionScript)

(fn Walk
  (Variables|Speed|SetTargetSpeed (Variables|Speed|GetWalkSpeed)))

(fn Run
  (Variables|Speed|SetTargetSpeed (Variables|Speed|GetRunSpeed)))

(fn RecoverStamina
  (Variables|Resource|SetStamina (Math|Float|Clamp(Float) (+ (Variables|Resource|GetStamina) (* (Utilities|Time|GetWorldDeltaSeconds) (Variables|Resource|GetStaminaRecoverRate))))))

(fn RecoverStaminaLogic
  (if (not (and (== (Variables|Speed|GetTargetSpeed) (Variables|Speed|GetRunSpeed)) (CallFunction|IsMoving)))
    (Recover|RecoverStamina)))

(fn LoseStaminaLogic
  (if (CallFunction|IsMoving)
    (Lose|LoseStamina)))

(fn LoseStamina
  (Variables|Resource|SetStamina (Math|Float|Clamp(Float) (+ (Variables|Resource|GetStamina) (* (Utilities|Time|GetWorldDeltaSeconds) (Variables|Resource|GetStaminaLostRate) -1.0)))))

(fn SmoothChangeMaxWalkSpeed
  (bind _charactermovement (Variables|Character|GetCharacterMovement))
  (Variables|/Script/Engine.CharacterMovementComponent|SetMaxWalkSpeed _charactermovement (Math|Float|Lerp (Variables|/Script/Engine.CharacterMovementComponent|GetMaxWalkSpeed _charactermovement) (Variables|Speed|GetTargetSpeed) 0.1)))

(fn GetAbsoluteVelocity
  (return (Math|Float|Absolute(Float) (Math|Vector|VectorLength (Variables|/Script/Engine.MovementComponent|GetVelocity (Variables|Character|GetCharacterMovement))))))

(fn IsMoving
  (return (> (CallFunction|GetAbsoluteVelocity) 0.0)))